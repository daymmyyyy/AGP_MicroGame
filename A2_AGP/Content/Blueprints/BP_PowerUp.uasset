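; Pickup actor for a two-player game that grants a random timed power-up to the character that overlaps it.
; Overlap plays a sound, then randomly boosts the collector's speed or jump, or slows the opponent found by player index.
; Each effect hides the Niagara effect, disables collision, then resets the stat to a hardcoded default after a delay and destroys the actor.
; A brief message appears in that player's widget text box.
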(event OnComponentBeginOverlap(CollisionComp)
  (params (OverlappedComponent :type Primitive%20Component%20Object%20Reference) (OtherActor :type Actor%20Object%20Reference) (OtherComp :type Primitive%20Component%20Object%20Reference) (OtherBodyIndex :type Integer) (bFromSweep :type Boolean) (SweepResult :type Hit%20Result%20Structure%20%28by%20ref%29))
  (Audio|PlaySound2D "/Game/Audio/collectcoin-6075.collectcoin-6075" 1.0 1.0 0.0 0 0)
  (bind _asbp_third_person_character (Utilities|Casting|CastToBP_ThirdPersonCharacter OtherActor))
  (Variables|Default|SetPlayerThatPickedUp _asbp_third_person_character)
  (switch int (Math|Random|RandomIntegerinRange 0 2)
    (:0
      (CallFunction|ApplySpeedBoost)
      (if (Variables|/Game/ThirdPerson/Blueprints/BP_ThirdPersonCharacter.BP_ThirdPersonCharacter_C|GetbIsPlayer1 _asbp_third_person_character)
        (Rendering|Components|TextRender|SetText (Variables|/Game/UI/W_PowerUp.W_PowerUp_C|GetPowerUpTextBox1 (Variables|/Game/ThirdPerson/Blueprints/BP_ThirdPersonCharacter.BP_ThirdPersonCharacter_C|GetPowerupWidgetRef (Variables|Default|GetPlayerThatPickedUp))) "speed boosted!")
        (Utilities|FlowControl|Delay 3.0)
        (Rendering|Components|TextRender|SetText (Variables|/Game/UI/W_PowerUp.W_PowerUp_C|GetPowerUpTextBox1 (Variables|/Game/ThirdPerson/Blueprints/BP_ThirdPersonCharacter.BP_ThirdPersonCharacter_C|GetPowerupWidgetRef (Variables|Default|GetPlayerThatPickedUp))) "")
        (else
          (Rendering|Components|TextRender|SetText (Variables|/Game/UI/W_PowerUp.W_PowerUp_C|GetPowerUpTextBox2 (Variables|/Game/ThirdPerson/Blueprints/BP_ThirdPersonCharacter.BP_ThirdPersonCharacter_C|GetPowerupWidgetRef (Variables|Default|GetPlayerThatPickedUp))) "speed boosted!")
          (Utilities|FlowControl|Delay 3.0)
          (Rendering|Components|TextRender|SetText (Variables|/Game/UI/W_PowerUp.W_PowerUp_C|GetPowerUpTextBox2 (Variables|/Game/ThirdPerson/Blueprints/BP_ThirdPersonCharacter.BP_ThirdPersonCharacter_C|GetPowerupWidgetRef (Variables|Default|GetPlayerThatPickedUp))) ""))))
    (:1
      (CallFunction|ApplyHighJump)
      (if (Variables|/Game/ThirdPerson/Blueprints/BP_ThirdPersonCharacter.BP_ThirdPersonCharacter_C|GetbIsPlayer1 _asbp_third_person_character)
        (Rendering|Components|TextRender|SetText (Variables|/Game/UI/W_PowerUp.W_PowerUp_C|GetPowerUpTextBox1 (Variables|/Game/ThirdPerson/Blueprints/BP_ThirdPersonCharacter.BP_ThirdPersonCharacter_C|GetPowerupWidgetRef (Variables|Default|GetPlayerThatPickedUp))) "high jump!")
        (Utilities|FlowControl|Delay 3.0)
        (Rendering|Components|TextRender|SetText (Variables|/Game/UI/W_PowerUp.W_PowerUp_C|GetPowerUpTextBox1 (Variables|/Game/ThirdPerson/Blueprints/BP_ThirdPersonCharacter.BP_ThirdPersonCharacter_C|GetPowerupWidgetRef (Variables|Default|GetPlayerThatPickedUp))) "")
        (else
          (Rendering|Components|TextRender|SetText (Variables|/Game/UI/W_PowerUp.W_PowerUp_C|GetPowerUpTextBox2 (Variables|/Game/ThirdPerson/Blueprints/BP_ThirdPersonCharacter.BP_ThirdPersonCharacter_C|GetPowerupWidgetRef (Variables|Default|GetPlayerThatPickedUp))) "high jump!")
          (Utilities|FlowControl|Delay 3.0)
          (Rendering|Components|TextRender|SetText (Variables|/Game/UI/W_PowerUp.W_PowerUp_C|GetPowerUpTextBox2 (Variables|/Game/ThirdPerson/Blueprints/BP_ThirdPersonCharacter.BP_ThirdPersonCharacter_C|GetPowerupWidgetRef (Variables|Default|GetPlayerThatPickedUp))) ""))))
    (:2
      (CallFunction|ApplySlowOpponent)
      (if (Variables|/Game/ThirdPerson/Blueprints/BP_ThirdPersonCharacter.BP_ThirdPersonCharacter_C|GetbIsPlayer1 _asbp_third_person_character)
        (Rendering|Components|TextRender|SetText (Variables|/Game/UI/W_PowerUp.W_PowerUp_C|GetPowerUpTextBox1 (Variables|/Game/ThirdPerson/Blueprints/BP_ThirdPersonCharacter.BP_ThirdPersonCharacter_C|GetPowerupWidgetRef (Variables|Default|GetPlayerThatPickedUp))) "opponent slowed!")
        (Utilities|FlowControl|Delay 3.0)
        (Rendering|Components|TextRender|SetText (Variables|/Game/UI/W_PowerUp.W_PowerUp_C|GetPowerUpTextBox1 (Variables|/Game/ThirdPerson/Blueprints/BP_ThirdPersonCharacter.BP_ThirdPersonCharacter_C|GetPowerupWidgetRef (Variables|Default|GetPlayerThatPickedUp))) "")
        (else
          (Rendering|Components|TextRender|SetText (Variables|/Game/UI/W_PowerUp.W_PowerUp_C|GetPowerUpTextBox2 (Variables|/Game/ThirdPerson/Blueprints/BP_ThirdPersonCharacter.BP_ThirdPersonCharacter_C|GetPowerupWidgetRef (Variables|Default|GetPlayerThatPickedUp))) "opponent slowed!")
          (Utilities|FlowControl|Delay 3.0)
          (Rendering|Components|TextRender|SetText (Variables|/Game/UI/W_PowerUp.W_PowerUp_C|GetPowerUpTextBox2 (Variables|/Game/ThirdPerson/Blueprints/BP_ThirdPersonCharacter.BP_ThirdPersonCharacter_C|GetPowerupWidgetRef (Variables|Default|GetPlayerThatPickedUp))) ""))))))

(event Custom|ApplyHighJump
  (Variables|/Script/Engine.CharacterMovementComponent|SetJumpZVelocity (Variables|/Script/Engine.Character|GetCharacterMovement (Variables|Default|GetPlayerThatPickedUp)) 1.2e+03)
  (Rendering|SetVisibility (Variables|Default|GetNiagara) false false)
  (Collision|SetCollisionEnabled (Variables|Default|GetCollisionComp) "NoCollision")
  (Utilities|FlowControl|Delay 5.0)
  (Variables|/Script/Engine.CharacterMovementComponent|SetJumpZVelocity (Variables|/Script/Engine.Character|GetCharacterMovement (Variables|Default|GetPlayerThatPickedUp)) 7e+02)
  (Actor|DestroyActor))

(event Custom|ApplySlowOpponent
  (if (== (Variables|/Game/ThirdPerson/Blueprints/BP_ThirdPersonCharacter.BP_ThirdPersonCharacter_C|GetControllerIndex (Variables|Default|GetPlayerThatPickedUp)) 0)
    (bind _asbp_third_person_character (Utilities|Casting|CastToBP_ThirdPersonCharacter (Game|GetPlayerCharacter 1)))
    (Variables|/Script/Engine.CharacterMovementComponent|SetMaxWalkSpeed (Variables|/Script/Engine.Character|GetCharacterMovement _asbp_third_person_character) 5e+02)
    (Rendering|SetVisibility (Variables|Default|GetNiagara) false false)
    (Collision|SetCollisionEnabled (Variables|Default|GetCollisionComp) "NoCollision")
    (Utilities|FlowControl|Delay 5.0)
    (Variables|/Script/Engine.CharacterMovementComponent|SetMaxWalkSpeed (Variables|/Script/Engine.Character|GetCharacterMovement _asbp_third_person_character) 8e+02)
    (Actor|DestroyActor)
    (else
      (bind _asbp_third_person_character_2 (Utilities|Casting|CastToBP_ThirdPersonCharacter (Game|GetPlayerCharacter 0)))
      (Variables|/Script/Engine.CharacterMovementComponent|SetMaxWalkSpeed (Variables|/Script/Engine.Character|GetCharacterMovement _asbp_third_person_character_2) 5e+02)
      (Rendering|SetVisibility (Variables|Default|GetNiagara) false false)
      (Collision|SetCollisionEnabled (Variables|Default|GetCollisionComp) "NoCollision")
      (Utilities|FlowControl|Delay 5.0)
      (Variables|/Script/Engine.CharacterMovementComponent|SetMaxWalkSpeed (Variables|/Script/Engine.Character|GetCharacterMovement _asbp_third_person_character_2) 8e+02)
      (Actor|DestroyActor))))

(event Custom|ApplySpeedBoost
  (Variables|/Script/Engine.CharacterMovementComponent|SetMaxWalkSpeed (Variables|/Script/Engine.Character|GetCharacterMovement (Variables|Default|GetPlayerThatPickedUp)) 1.5e+03)
  (Rendering|SetVisibility (Variables|Default|GetNiagara) false false)
  (Collision|SetCollisionEnabled (Variables|Default|GetCollisionComp) "NoCollision")
  (Utilities|FlowControl|Delay 5.0)
  (Variables|/Script/Engine.CharacterMovementComponent|SetMaxWalkSpeed (Variables|/Script/Engine.Character|GetCharacterMovement (Variables|Default|GetPlayerThatPickedUp)) 8e+02)
  (Actor|DestroyActor))

(fn ConstructionScript)