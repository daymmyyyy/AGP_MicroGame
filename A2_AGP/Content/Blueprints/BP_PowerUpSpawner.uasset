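; Spawner actor that scatters a set number of BP_PowerUp pickups across a rectangular area when play begins.
; On BeginPlay it reads the locations of StartActor and EndActor as opposite corners of the area.
; It then spawns PowerUpCount power-ups at random X and Y between those corners, at a fixed height with no rotation.
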(event EventBeginPlay
  (bind _output_get (Variables|Default|SetStartLocation (Transformation|GetActorLocation (Variables|Default|GetStartActor))))
  (bind _output_get_2 (Variables|Default|SetEndLocation (Transformation|GetActorLocation (Variables|Default|GetEndActor))))
  (for _index (range 0 (- (Variables|Default|GetPowerUpCount) 1))
    (Game|SpawnActorfromClass "/Game/Blueprints/BP_PowerUp.BP_PowerUp_C" (Math|Transform|MakeTransform (Math|Vector|MakeVector (Math|Random|RandomFloatinRange (.X (Math|Vector|BreakVector _output_get)) (.X (Math|Vector|BreakVector _output_get_2))) (Math|Random|RandomFloatinRange (.Y (Math|Vector|BreakVector _output_get)) (.Y (Math|Vector|BreakVector _output_get_2))) 1.5e+02)) "Undefined" "MultiplyWithRoot" 0 0)))

(fn ConstructionScript)