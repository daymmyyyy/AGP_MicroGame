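; Finish-line trigger that records player 2's completion in a timed race.
; When a third-person character with a controller index above zero overlaps the box, it pauses that character's second timer and disables its movement.
; It then copies the speedrun time from the character's timer widget into the game mode, flags player 2 as finished and asks the game mode to check whether players have finished.
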(event OnComponentBeginOverlap(Box)
  (params (OverlappedComponent :type Primitive%20Component%20Object%20Reference) (OtherActor :type Actor%20Object%20Reference) (OtherComp :type Primitive%20Component%20Object%20Reference) (OtherBodyIndex :type Integer) (bFromSweep :type Boolean) (SweepResult :type Hit%20Result%20Structure%20%28by%20ref%29))
  (bind _asbp_third_person_character (Utilities|Casting|CastToBP_ThirdPersonCharacter OtherActor))
  (if (> (Variables|/Game/ThirdPerson/Blueprints/BP_ThirdPersonCharacter.BP_ThirdPersonCharacter_C|GetControllerIndex _asbp_third_person_character) 0)
    (Variables|/Game/ThirdPerson/Blueprints/BP_ThirdPersonCharacter.BP_ThirdPersonCharacter_C|SetPauseTimer2 _asbp_third_person_character true)
    (Pawn|Components|CharacterMovement|DisableMovement (Variables|/Script/Engine.Character|GetCharacterMovement _asbp_third_person_character))
    (bind _asbp_third_person_game_mode (Utilities|Casting|CastToBP_ThirdPersonGameMode (Game|GetGameMode)))
    (Variables|/Game/ThirdPerson/Blueprints/BP_ThirdPersonGameMode.BP_ThirdPersonGameMode_C|SetPlayer2Time _asbp_third_person_game_mode (Variables|/Game/UI/W_Timer1.W_Timer1_C|GetSpeedRunTimer (Variables|/Game/ThirdPerson/Blueprints/BP_ThirdPersonCharacter.BP_ThirdPersonCharacter_C|GetTimerWidgetRef1 _asbp_third_person_character)))
    (Variables|/Game/ThirdPerson/Blueprints/BP_ThirdPersonGameMode.BP_ThirdPersonGameMode_C|SetbPlayer2Finished? _asbp_third_person_game_mode true)
    (Development|PrintString "player 2 finished")
    (Default|CheckPlayersFinished _asbp_third_person_game_mode)))

(fn ConstructionScript)